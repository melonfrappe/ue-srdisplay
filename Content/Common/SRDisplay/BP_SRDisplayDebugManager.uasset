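; Debug display actor for SRDisplay that shows the average frame rate as in-world text.
; The construction script applies the configured text color to the FPS text render component.
; Every tick, UpdatePerformance reads the average FPS and writes it to that component with an "FPS:" prefix.
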(event `self.ReceiveTick`
  (params (DeltaSeconds :type "Float (single-precision)"))
  (`self.UpdatePerformance` DeltaSeconds))

(fn `UpdatePerformance`
  (params (`Delta Time` :type "Float (double-precision)"))
  (bind _returnvalue (`SampleBlueprintFunctionLibrary.GetAverageFps`))
  (`TextRenderComponent.K2_SetText` (`self.FPS`) (`KismetTextLibrary.Conv_StringToText` (`KismetStringLibrary.Concat_StrStr` "FPS: " (`KismetTextLibrary.Conv_TextToString` (`KismetTextLibrary.Conv_DoubleToText` _returnvalue "HalfToEven" false true 1 4 1 1))))))

(fn `UserConstructionScript`
  (`TextRenderComponent.SetTextRenderColor` (`self.FPS`) (`self.TextColor`)))