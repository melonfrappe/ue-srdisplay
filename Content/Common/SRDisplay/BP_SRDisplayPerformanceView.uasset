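; BP_SRDisplayPerformanceView is an FPS readout for the SRDisplay performance view.
; Each Tick passes the frame delta to UpdatePerformance, which accumulates elapsed time and refreshes the FPS text about every tenth of a second.
; The displayed value is the inverse of the current frame's delta, so it is an instantaneous sample rather than an average over the interval.
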(event `self.ReceiveTick`
  (params (DeltaSeconds :type "Float (single-precision)"))
  (`self.UpdatePerformance` DeltaSeconds))

(fn `UpdatePerformance`
  (params (DeltaTime :type "Float (double-precision)"))
  (bind _output_get (set `self.ElapsedTime` (+ DeltaTime (`self.ElapsedTime`))))
  (if (>= _output_get 0.1)
    (set `self.ElapsedTime` 0.0)
    (`TextRenderComponent.K2_SetText` (`self.FPS`) (`KismetTextLibrary.Conv_StringToText` (`KismetStringLibrary.Concat_StrStr` "FPS: " (`KismetTextLibrary.Conv_TextToString` (`KismetTextLibrary.Conv_DoubleToText` (/ 1.0 DeltaTime) "HalfToEven" false true 1 4 1 1)))))))

(fn `UserConstructionScript`)