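; BP_DragAndDropCube is a cube actor that can be dragged with the left mouse button and turns emerald green while held, gray on release.
; On press, Clicked runs a short Visibility line trace from the deprojected mouse position to confirm this actor was hit.
; While held, Tick moves the cube by the change in mouse world position, scaled by SpeedCorrectionValue, as an unswept local offset.
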(event `Key|LeftMouseButton` :consume false
  (params (Key :type "Key Structure"))
  (:`Pressed`
    (bind _returnvalue (`self.Clicked`))
    (if _returnvalue
      (set `self.IsClicked` true)
      (set `self.OldMouseWorldPosition` (`SRDisplayFunctionLibrary.ConvertMouseLocationToWorldSpace` (`GameplayStatics.GetPlayerController` 0)))
      (`PrimitiveComponent.SetMaterial` (`self.Cube`) 0 "/Game/DragAndDrop/Materials/M_EmeraldGreen.M_EmeraldGreen")))
  (:`Released`
    (set `self.IsClicked` false)
    (`PrimitiveComponent.SetMaterial` (`self.Cube`) 0 "/Game/DragAndDrop/Materials/M_Gray.M_Gray")))

(event `self.ReceiveTick`
  (params (DeltaSeconds :type "Float (single-precision)"))
  (bind (_worldposition _worlddirection _returnvalue) (`SRDisplayFunctionLibrary.ConvertMouseLocationToWorldSpace` (`GameplayStatics.GetPlayerController` 0)))
  (if (`self.IsClicked`)
    (if _returnvalue
      (`self.K2_AddActorLocalOffset` (* (- _worldposition (`self.OldMouseWorldPosition`)) (`self.SpeedCorrectionValue`)))
      (set `self.OldMouseWorldPosition` _worldposition))))

(fn `Clicked`
  (returns (ReturnValue :type Boolean))
  (bind (_worldposition _worlddirection _returnvalue) (`SRDisplayFunctionLibrary.ConvertMouseLocationToWorldSpace` (`GameplayStatics.GetPlayerController` 0)))
  (if _returnvalue
    (bind (_outhit _returnvalue_2) (`KismetSystemLibrary.LineTraceSingle` :`Start` _worldposition :`End` (+ _worldposition (* _worlddirection 200.0)) :`TraceChannel` "TraceTypeQuery1" :`bIgnoreSelf` false))
    (if _returnvalue_2
      (return (== self (`.HitActor` (`GameplayStatics.BreakHitResult` _outhit))))
      (else
        _)))
  (return false))

(fn `UserConstructionScript`)