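; BP_MouseCursor is an actor that acts as a 3D mouse cursor, moving a sphere through the world to follow the player's mouse.
; The sphere starts hidden and appears once the mouse location first converts to world space.
; Each tick, it traces on the Visibility channel from the camera along the mouse direction.
; The actor snaps to the impact point, or to the mouse's world position if nothing is hit within range.
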(event `self.ReceiveBeginPlay`
  (`SceneComponent.SetVisibility` (`self.Sphere`) false false))

(event `self.ReceiveTick`
  (params (DeltaSeconds :type "Float (single-precision)"))
  (bind _sphere (`self.Sphere`))
  (bind _cameraposition (`self.CameraPosition`))
  (bind (_worldposition _worlddirection _cameraposition_2 _returnvalue) (`SRDisplayFunctionLibrary.ConvertMouseLocationToWorldSpace` (`GameplayStatics.GetPlayerController` 0)))
  (if _returnvalue
    (set `self.MousePosition` _worldposition)
    (set `self.MouseDirection` _worlddirection)
    (set `self.CameraPosition` _cameraposition_2)
    (if (not (`SceneComponent.IsVisible` _sphere))
      (`SceneComponent.SetVisibility` _sphere true false))
    (bind (_outhit _returnvalue_2) (`KismetSystemLibrary.LineTraceSingle` _cameraposition (+ _cameraposition (* (`self.MouseDirection`) 1000.0)) "TraceTypeQuery1"))
    (if _returnvalue_2
      (`self.K2_SetActorLocation` (`.ImpactPoint` (`GameplayStatics.BreakHitResult` _outhit)))
      (else
        (`self.K2_SetActorLocation` (`self.MousePosition`))))))

(fn `UserConstructionScript`)