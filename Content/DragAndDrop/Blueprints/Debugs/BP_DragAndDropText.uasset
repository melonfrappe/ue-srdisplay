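; Debug Blueprint for drag and drop that shows mouse click coordinates and their world-space projection as text.
; On a left mouse press with a valid cursor position, it writes the screen position to the Coordinate text.
; It deprojects that position through player controller 0, writing the world origin to LocationStart and a point 1000 units along the ray to LocationEnd.
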(event `Key|LeftMouseButton` :consume false
  (params (Key :type "Key Structure"))
  (bind (_locationx _locationy _returnvalue) (`SRDisplayFunctionLibrary.GetMousePosition`))
  (bind _returnvalue_2 (`KismetMathLibrary.MakeVector2D` _locationx _locationy))
  (bind (_worldposition _worlddirection) (`SRDisplayFunctionLibrary.DeprojectScreenToWorld` (`GameplayStatics.GetPlayerController` 0) _returnvalue_2))
  (:`Pressed`
    (if _returnvalue
      (`TextRenderComponent.K2_SetText` (`self.Coordinate`) (`KismetTextLibrary.Conv_Vector2dToText` _returnvalue_2))
      (if true
        (`TextRenderComponent.K2_SetText` (`self.LocationStart`) (`KismetTextLibrary.Conv_VectorToText` _worldposition))
        (`TextRenderComponent.K2_SetText` (`self.LocationEnd`) (`KismetTextLibrary.Conv_VectorToText` (+ _worldposition (* _worlddirection 1000.0))))))))

(fn `UserConstructionScript`)