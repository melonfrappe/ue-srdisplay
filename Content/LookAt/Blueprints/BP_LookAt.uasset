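; BP_LookAt is a Blueprint that turns its Head component to face a tracked XR device.
; Each tick it reads the pose of the first enumerated device of any type and, if tracked, computes a look-at rotation toward that position.
; RInterpTo eases the Head's world rotation toward that target at RInterpSpeed, using the device position directly as a world-space point.
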(event `self.ReceiveTick`
  (params (DeltaSeconds :type "Float (single-precision)"))
  ;[1 1 1] LookAt Tracking Info
  (bind _returnvalue (`HeadMountedDisplayFunctionLibrary.EnumerateTrackedDevices` "None"))
  (bind (_bistracked _orientation _bhaspositionaltracking _position) (`HeadMountedDisplayFunctionLibrary.GetDevicePose` (`|GetArrayItem` _returnvalue)))
  (if _bistracked
    (`SceneComponent.K2_SetWorldRotation` (`self.Head`) (`KismetMathLibrary.RInterpTo` (`SceneComponent.K2_GetComponentRotation` (`self.Head`)) (`KismetMathLibrary.FindLookAtRotation` (`SceneComponent.K2_GetComponentLocation` (`self.Head`)) _position) DeltaSeconds (`self.RInterpSpeed`)) false false)))

(fn `UserConstructionScript`)