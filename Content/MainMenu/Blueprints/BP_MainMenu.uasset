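; BP_MainMenu is a main menu that lets the player pick a level with the keyboard.
; On BeginPlay it fills five text render items with names from LevelNameArray and collects them in MenuItemArray.
; Up and Down move ItemIndex with wraparound, then SetMenuColor highlights the selected item green and the rest white.
; Enter calls SwitchLevel with the selected name.
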(event `self.ReceiveBeginPlay`
  (bind _textrender_item03 (`self.TextRender-Item03`))
  (bind _textrender_item01 (`self.TextRender-Item01`))
  (bind _textrender_item02 (`self.TextRender-Item02`))
  (bind _textrender_item04 (`self.TextRender-Item04`))
  (bind _textrender_item00 (`self.TextRender-Item00`))
  (`KismetArrayLibrary.Array_Add` (`self.MenuItemArray`) _textrender_item00)
  (`TextRenderComponent.K2_SetText` _textrender_item00 (`KismetTextLibrary.Conv_NameToText` (`|GetArrayItem` (`self.LevelNameArray`))))
  (`KismetArrayLibrary.Array_Add` (`self.MenuItemArray`) _textrender_item01)
  (`TextRenderComponent.K2_SetText` _textrender_item01 (`KismetTextLibrary.Conv_NameToText` (`|GetArrayItem` (`self.LevelNameArray`) 1)))
  (`KismetArrayLibrary.Array_Add` (`self.MenuItemArray`) _textrender_item02)
  (`TextRenderComponent.K2_SetText` _textrender_item02 (`KismetTextLibrary.Conv_NameToText` (`|GetArrayItem` (`self.LevelNameArray`) 2)))
  (`KismetArrayLibrary.Array_Add` (`self.MenuItemArray`) _textrender_item03)
  (`TextRenderComponent.K2_SetText` _textrender_item03 (`KismetTextLibrary.Conv_NameToText` (`|GetArrayItem` (`self.LevelNameArray`) 3)))
  (`KismetArrayLibrary.Array_Add` (`self.MenuItemArray`) _textrender_item04)
  (`TextRenderComponent.K2_SetText` _textrender_item04 (`KismetTextLibrary.Conv_NameToText` (`|GetArrayItem` (`self.LevelNameArray`) 4)))
  (`self.SetMenuColor`))

(event `Key|Down`
  (params (Key :type "Key Structure"))
  (:`Pressed`
    (bind _result (`/Engine/EditorBlueprintResources/StandardMacros.IncrementInt` (`self.ItemIndex`))
      (:`  `
        (if (>= _result (`KismetArrayLibrary.Array_Length` (`self.LevelNameArray`)))
          (set `self.ItemIndex` 0))
        (`self.SetMenuColor`)))))

(event `Key|Up`
  (params (Key :type "Key Structure"))
  (:`Pressed`
    (bind _result (`/Engine/EditorBlueprintResources/StandardMacros.DecrementInt` (`self.ItemIndex`))
      (:`  `
        (if (< _result 0)
          (set `self.ItemIndex` (- (`KismetArrayLibrary.Array_Length` (`self.LevelNameArray`)) 1)))
        (`self.SetMenuColor`)))))

(event `Key|Enter`
  (params (Key :type "Key Structure"))
  (:`Pressed`
    (`/Game/Common/SRDisplay/BML_LevelSwitching.SwitchLevel` (`|GetArrayItem` (`self.LevelNameArray`) (`self.ItemIndex`)))))

(fn `SetMenuColor`
  (for (_array_element _array_index) (`self.MenuItemArray`)
    (if (== _array_index (`self.ItemIndex`))
      (`TextRenderComponent.SetTextRenderColor` _array_element (make `Color` 0 255))
      (else
        (`TextRenderComponent.SetTextRenderColor` _array_element (make `Color` 255 255 255))))))

(fn `UserConstructionScript`)