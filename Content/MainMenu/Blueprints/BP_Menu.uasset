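; BP_Menu is a level-select main menu actor that shows level names as 3D text render components.
; BeginPlay fills four text items from LevelNameArray and registers them in MenuItemArray.
; Up and Down keys move the selection with wraparound, and SetMenuColor tints the selected item green and the rest white.
; Enter opens the selected level by name.
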(event `self.ReceiveBeginPlay`
  (bind _textrender_menu00 (`self.TextRender-Menu00`))
  (bind _textrender_menu02 (`self.TextRender-Menu02`))
  (bind _textrender_menu03 (`self.TextRender-Menu03`))
  (bind _textrender_menu01 (`self.TextRender-Menu01`))
  (`KismetArrayLibrary.Array_Add` (`self.MenuItemArray`) _textrender_menu00)
  (`TextRenderComponent.K2_SetText` _textrender_menu00 (`KismetTextLibrary.Conv_NameToText` (`|GetArrayItem` (`self.LevelNameArray`))))
  (`KismetArrayLibrary.Array_Add` (`self.MenuItemArray`) _textrender_menu01)
  (`TextRenderComponent.K2_SetText` _textrender_menu01 (`KismetTextLibrary.Conv_NameToText` (`|GetArrayItem` (`self.LevelNameArray`) 1)))
  (`KismetArrayLibrary.Array_Add` (`self.MenuItemArray`) _textrender_menu02)
  (`TextRenderComponent.K2_SetText` _textrender_menu02 (`KismetTextLibrary.Conv_NameToText` (`|GetArrayItem` (`self.LevelNameArray`) 2)))
  (`KismetArrayLibrary.Array_Add` (`self.MenuItemArray`) _textrender_menu03)
  (`TextRenderComponent.K2_SetText` _textrender_menu03 (`KismetTextLibrary.Conv_NameToText` (`|GetArrayItem` (`self.LevelNameArray`) 3)))
  (`self.SetMenuColor`))

(event `Key|Down`
  (params (Key :type "Key Structure"))
  (:`Pressed`
    (bind _result (`/Engine/EditorBlueprintResources/StandardMacros.IncrementInt` (`self.SelectedItemIndex`))
      (:`  `
        (if (>= _result (`KismetArrayLibrary.Array_Length` (`self.LevelNameArray`)))
          (set `self.SelectedItemIndex` 0))
        (`self.SetMenuColor`)))))

(event `Key|Up`
  (params (Key :type "Key Structure"))
  (:`Pressed`
    (bind _result (`/Engine/EditorBlueprintResources/StandardMacros.DecrementInt` (`self.SelectedItemIndex`))
      (:`  `
        (if (< _result 0)
          (set `self.SelectedItemIndex` (- (`KismetArrayLibrary.Array_Length` (`self.LevelNameArray`)) 1)))
        (`self.SetMenuColor`)))))

(event `Key|Enter`
  (params (Key :type "Key Structure"))
  (:`Pressed`
    (`GameplayStatics.OpenLevel` (`|GetArrayItem` (`self.LevelNameArray`) (`self.SelectedItemIndex`)))))

(fn `SetMenuColor`
  (for (_array_element _array_index) (`self.MenuItemArray`)
    (if (== _array_index (`self.SelectedItemIndex`))
      (`TextRenderComponent.SetTextRenderColor` _array_element (make `Color` 0 255))
      (else
        (`TextRenderComponent.SetTextRenderColor` _array_element (make `Color` 255 255 255))))))

(fn `UserConstructionScript`)