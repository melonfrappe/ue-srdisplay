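; DynamicContextBP is a Blueprint that hosts a DynamicContextWidgetBP in a widget component to display contextual information with a progress bar.
; On BeginPlay it passes its Context value to the widget and caches the widget's progress bar.
; SetContext writes a new context to the widget, and SetProgress updates the cached bar's percent.
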(event `self.ReceiveBeginPlay`
  (bind _asdynamic_context_widget_bp (cast `/Game/_Blueprints/DynamicContextWidgetBP` (`WidgetComponent.GetWidget` (`self.Widget`))))
  (set `/Game/_Blueprints/DynamicContextWidgetBP.Context` (`self.Context`) _asdynamic_context_widget_bp)
  (set `self.Progress Bar` (`/Game/_Blueprints/DynamicContextWidgetBP.ProgressBar_0` _asdynamic_context_widget_bp)))

(event `SetContext`
  (params (Context :type Text))
  (bind _asdynamic_context_widget_bp (cast `/Game/_Blueprints/DynamicContextWidgetBP` (`WidgetComponent.GetWidget` (`self.Widget`))))
  (set `/Game/_Blueprints/DynamicContextWidgetBP.Context` Context _asdynamic_context_widget_bp))

(event `Set Progress`
  (params (InPercent :type "Float (double-precision)"))
  (`ProgressBar.SetPercent` (`self.Progress Bar`) InPercent))

(fn `UserConstructionScript`)