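; Importer Blueprint that loads a hard-coded test static mesh at runtime and fits it to a reference size.
; On BeginPlay it async-loads the mesh from a soft object path and assigns it to the Parent actor's StaticMeshComponent.
; It then uniformly scales Parent by the ratio of the MaxBound actor's local X bound to the loaded mesh's X extent, matching on that axis only.
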(event `self.ReceiveBeginPlay`
  (bind _parent (`self.parent`))
  (bind _object (`|LoadAsset` (`KismetSystemLibrary.Conv_SoftObjPathToSoftObjRef` (`KismetSystemLibrary.MakeSoftObjectPath` "StaticMesh'/Game/_Meshes/_test/0/oniyuri.oniyuri'")))
    (:`Completed`
      (bind _asstatic_mesh (cast `StaticMesh` _object))
      (`StaticMeshComponent.SetStaticMesh` (`StaticMeshActor.StaticMeshComponent` _parent) _asstatic_mesh)
      (`self.SetActorScale3D` _parent (`KismetMathLibrary.Conv_DoubleToVector` (/ (.x (`.Max` (`StaticMeshComponent.GetLocalBounds` (`StaticMeshActor.StaticMeshComponent` (`self.maxBound`))))) (.x (`.BoxExtent` (`KismetMathLibrary.BreakBoxSphereBounds` (`StaticMesh.GetBounds` _asstatic_mesh))))))))))

(fn `UserConstructionScript`)