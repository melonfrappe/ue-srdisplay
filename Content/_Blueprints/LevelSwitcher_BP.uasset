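; LevelSwitcher_BP switches the game to another level from a key, choosing among several project versions built around sites such as Yoshino, Saigai and Kitanaikaku.
; SwitchLevelbyKey reloads the current level when IsReloadCurrentLevel is set.
; Otherwise it selects the active Version by CurrentVersionIndex and looks the key up in that version's own level map.
; A found entry is passed to SwitchLevel, while a missing key does nothing.
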(event `Switch Level by Key`
  (params (Key :type "Key Structure (by ref)"))
  (bind (_value _returnvalue) (`BlueprintMapLibrary.Map_Find` (`self.Level Map_0`) Key))
  (bind (_value_2 _returnvalue_2) (`BlueprintMapLibrary.Map_Find` (`self.Level Map_5`) Key))
  (bind (_value_3 _returnvalue_3) (`BlueprintMapLibrary.Map_Find` (`self.Level Map_1`) Key))
  (bind (_value_4 _returnvalue_4) (`BlueprintMapLibrary.Map_Find` (`self.Level Map_2`) Key))
  (bind (_value_5 _returnvalue_5) (`BlueprintMapLibrary.Map_Find` (`self.Level Map_3`) Key))
  (bind (_value_6 _returnvalue_6) (`BlueprintMapLibrary.Map_Find` (`self.Level Map_4`) Key))
  (if (`self.isReloadCurrentLevel?`)
    (bind _returnvalue_7 (`GameplayStatics.GetCurrentLevelName` true))
    (`/Game/Common/SRDisplay/BML_LevelSwitching.SwitchLevel` (`KismetStringLibrary.Conv_StringToName` _returnvalue_7))
    (else
      (switch `name` (`|GetArrayItem` (`self.version`) (`self.currentVersionIndex`))
        (:`yoshino-saigai-plateau-bim`
          ;[1 1 1] 0
          (if _returnvalue
            (`/Game/Common/SRDisplay/BML_LevelSwitching.SwitchLevel` _value)))
        (:`yoshino-saigai-plateau`
          ;[1 1 1] 1
          (if _returnvalue_3
            (`/Game/Common/SRDisplay/BML_LevelSwitching.SwitchLevel` _value_3)))
        (:`saigai-plateau`
          ;[1 1 1] 2
          (if _returnvalue_4
            (`/Game/Common/SRDisplay/BML_LevelSwitching.SwitchLevel` _value_4)))
        (:`kitanaikaku-kamekan-bim`
          ;[1 1 1] 3
          (if _returnvalue_5
            (`/Game/Common/SRDisplay/BML_LevelSwitching.SwitchLevel` _value_5)))
        (:`kitanaikaku-yoneda`
          ;[1 1 1] 4
          (if _returnvalue_6
            (`/Game/Common/SRDisplay/BML_LevelSwitching.SwitchLevel` _value_6)))
        (:`kitanaikaku-yachiyoza-plateau-bim`
          ;[1 1 1] 5
          (if _returnvalue_2
            (`/Game/Common/SRDisplay/BML_LevelSwitching.SwitchLevel` _value_2)))))))

(fn `UserConstructionScript`)