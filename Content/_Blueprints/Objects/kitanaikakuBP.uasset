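; Scripted sequence Blueprint that animates two target actors and then switches to the "kamekan" level.
; On BeginPlay it stores both actors' transforms, waits briefly, then runs DoMove.
; A first timeline drives the location, yaw and scale of Target, and on finish a second timeline rotates Target0 before the level switch.
; Separate events restore the saved transforms and stop or reset each timeline.
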(event `self.ReceiveBeginPlay`
  ;[1 1 1] Comment
  (set `self.NewVar_0` (`self.GetTransform` (`self.target`)))
  (set `self.NewVar_1` (`self.GetTransform` (`self.target_0`)))
  (`KismetSystemLibrary.Delay` 1.0)
  (`self.Do Move`))

(event `Set Default`
  ;[1 1 1] Comment
  (`self.K2_SetActorTransform` (`self.target`) (`self.NewVar_0`) false false)
  (`self.K2_SetActorTransform` (`self.target_0`) (`self.NewVar_1`) false false))

(event `Do Move`
  ;[1 1 1] Comment
  (bind (_direction _location _rotation _scale) (`Timeline|Timeline_0` :!label _label)
    (:`Update`
      (bind _returnvalue (`KismetMathLibrary.Conv_DoubleToVector` _scale))
      (`self.K2_SetActorTransform` (`self.target`) (`KismetMathLibrary.MakeTransform` _location (`KismetMathLibrary.MakeRotator` 0.0 0.0 _rotation) _returnvalue) false false)
      (set `self.Delta Scale` _returnvalue))
    (:`Finished`
      (bind (_direction_2 _rotation_2) (`Timeline|Timeline_1` :!label _label_2)
        (:`Update`
          (`self.K2_SetActorRotation` (`self.target_0`) (`KismetMathLibrary.MakeRotator` 0.0 0.0 _rotation_2) false))
        (:`Finished`
          (`/Game/Common/SRDisplay/BML_LevelSwitching.SwitchLevel` "kamekan"))))))

(event `Stop 0`
  ;[1 1 1] Comment
  (goto _label :!via `Stop`))

(event `Reset 0`
  ;[1 1 1] Comment
  (goto _label :!via `SetNewTime`))

(event `Stop 1`
  ;[1 1 1] Comment
  (goto _label_2 :!via `Stop`))

(event `Reset 1`
  ;[1 1 1] Comment
  (goto _label_2 :!via `SetNewTime`))

(fn `UserConstructionScript`)