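; Blueprint that animates a Target actor's transform with a timeline, then loads the "sagara" level when it finishes.
; BeginPlay stores the target's starting transform, waits briefly, then calls DoMove, whose timeline drives location, rotation and uniform scale each update.
; Stop, Reset and SetDefault events halt the timeline, set its time, or restore the saved transform; some leftover toggle logic is unconnected.
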(event `self.ReceiveBeginPlay`
  ;[1 1 1] Comment
  (set `self.NewVar_0` (`self.GetTransform` (`self.target`)))
  (`KismetSystemLibrary.Delay` 1.0)
  (`self.Do Move`))

(event `Do Move`
  (bind (_direction _rotation _location _scale) (`Timeline|Timeline_0` :!label _label)
    (:`Update`
      (bind _output_get (set `self.Delta Scale` (`KismetMathLibrary.Conv_DoubleToVector` _scale)))
      (`self.K2_SetActorTransform` (`self.target`) (`KismetMathLibrary.MakeTransform` _location (`KismetMathLibrary.MakeRotator` 0.0 (.y _rotation) (.z _rotation)) _output_get) false false))
    (:`Finished`
      (`/Game/Common/SRDisplay/BML_LevelSwitching.SwitchLevel` "sagara"))))

(event `Stop`
  (goto _label :!via `Stop`))

(event `Reset`
  (goto _label :!via `SetNewTime`))

(event `Set Default`
  ;[1 1 1] Comment
  (`self.K2_SetActorTransform` (`self.target`) (`self.NewVar_0`) false false))

(fn `UserConstructionScript`)