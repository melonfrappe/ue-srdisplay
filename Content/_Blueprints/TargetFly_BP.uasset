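; TargetFly_BP is a Blueprint that moves, rotates and scales a target actor through a DoTransform event.
; DoTransform applies a location delta along the actor's forward, right and up vectors, adds world rotation, and sets scale as an offset from the scale cached at BeginPlay.
; Tick clamps pitch to a limited nose-up range while keeping the current yaw.
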(event `self.ReceiveBeginPlay`
  ;[1 1 1] default
  (set `self.currentScale` (`self.GetActorScale3D` (`self.target`))))

(event `Do Transform`
  (params (DeltaLocation :type "Vector Structure") (DeltaRotation :type "Rotator Structure") (NewScale3D :type "Vector Structure"))
  (bind _target (`self.Target`))
  (bind _target_2 (`self.Target`))
  ;[1 1 1] controller
  (`self.K2_AddActorWorldOffset` _target_2 (+ (* (`self.GetActorForwardVector` _target_2) DeltaLocation_X) (* (`self.GetActorRightVector` _target_2) DeltaLocation_Y) (* (`self.GetActorUpVector` _target_2) DeltaLocation_Z)) false false)
  (`self.K2_AddActorWorldRotation` _target DeltaRotation false false)
  (`self.SetActorScale3D` _target (+ NewScale3D (`self.currentScale`))))

(event `self.ReceiveTick`
  (params (DeltaSeconds :type "Float (single-precision)"))
  (bind _target (`self.target`))
  (bind (_returnvalue_roll _returnvalue_pitch _returnvalue_yaw) (`KismetMathLibrary.BreakRotator` (`self.K2_GetActorRotation` _target)))
  ;[1 1 1] tick
  (`self.K2_SetActorRotation` _target (`KismetMathLibrary.MakeRotator` 0.0 (`KismetMathLibrary.ClampAngle` _returnvalue_pitch 0.0 30.0) _returnvalue_yaw) false))

(fn `UserConstructionScript`)