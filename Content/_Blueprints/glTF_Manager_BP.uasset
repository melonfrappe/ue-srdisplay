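; Manager Blueprint that prepares imported Datasmith scene actors, apparently glTF models, for display under a shared Parent actor.
; On BeginPlay, Init makes each actor movable, hides child meshes named "Cube", shows only the first actor's remaining meshes and attaches everything to Parent.
; It fits each model to the MaxBound actor's position and size using a ratio of bounds vector lengths.
; ResetTransform restores Parent's mesh to the transform cached at startup.
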(event `self.ReceiveBeginPlay`
  ;[1 1 1] begin
  (`self.Init`)
  (set `self.defaultTransform` (`self.GetTransform` (`self.parent`))))

(event `Reset Transform`
  ;[1 1 1] reset transform
  (`SceneComponent.K2_SetWorldTransform` (`StaticMeshActor.StaticMeshComponent` (`self.parent`)) (`self.defaultTransform`) false false))

(event `Init`
  (bind _maxbound (`self.maxBound`))
  ;[1 1 1] init
  (for (_array_element _array_index) (`self.datasmithSceneActor`)
    (`|ExecutionSequence`
      (:`then_0`
        (`SceneComponent.SetMobility` (`self.GetComponentByClass` _array_element "/Script/Engine.SceneComponent") "Movable"))
      (:`then_1`
        (for _array_element_2 (`self.GetAttachedActors` _array_element true)
          (bind _asstatic_mesh_actor (cast `StaticMeshActor` _array_element_2))
          (if (`KismetStringLibrary.Contains` (`KismetSystemLibrary.GetObjectName` _asstatic_mesh_actor) "Cube")
            (`self.SetActorHiddenInGame` _asstatic_mesh_actor true)
            (else
              (`self.K2_SetActorTransform` _array_element (`KismetMathLibrary.MakeTransform` (`self.K2_GetActorLocation` _maxbound) (struct :`Yaw` 90.0) (`KismetMathLibrary.Conv_DoubleToVector` (/ (`KismetMathLibrary.VSize` (`.Max` (`StaticMeshComponent.GetLocalBounds` (`StaticMeshActor.StaticMeshComponent` _maxbound)))) (`KismetMathLibrary.VSize` (`.Max` (`StaticMeshComponent.GetLocalBounds` (`StaticMeshActor.StaticMeshComponent` _asstatic_mesh_actor))))))) false false)
              (`self.SetActorHiddenInGame` _asstatic_mesh_actor (not (== _array_index 0)))))))
      (:`then_2`
        (`self.K2_AttachToActor` _array_element (`self.parent`) "None" "KeepWorld" "KeepWorld" "KeepWorld" true)))))

(fn `UserConstructionScript`)