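; BIM animation Blueprint that plays a building animation in the BIM map, then switches to the "kitanaikaku" level when it finishes.
; DoMove alternates between playing and stopping a timeline that drives the Root actor's yaw, X/Z location and uniform scale, plus the Mask's relative height.
; Root's starting transform is cached on BeginPlay, and separate events restore that transform or rewind the timeline.
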(event `self.ReceiveBeginPlay`
  (set `self.DEFAULT` (`self.GetTransform` (`self.Root`))))

(event `Reset Transform`
  (`self.K2_SetActorTransform` (`self.Root`) (`self.DEFAULT`) false false))

(event `DoMove`
  (bind _root (`self.Root`))
  (`/Engine/EditorBlueprintResources/StandardMacros.FlipFlop`
    (:`A`
      (bind (_direction _building_rotation _building_location_z _building_location_x _building_size _mask_location_z) (`Timeline|Timeline_0` :!label _label)
        (:`Update`
          (`SceneComponent.K2_SetWorldRotation` (`StaticMeshActor.StaticMeshComponent` _root) (`KismetMathLibrary.MakeRotator` 0.0 0.0 _building_rotation) false false)
          (`self.K2_SetActorLocation` _root (`KismetMathLibrary.MakeVector` _building_location_x -5.0 _building_location_z) false false)
          (`self.SetActorScale3D` _root (`KismetMathLibrary.Conv_DoubleToVector` _building_size))
          (`self.K2_SetActorRelativeLocation` (`self.Mask`) (`KismetMathLibrary.MakeVector` 0.0 0.0 _mask_location_z) false false))
        (:`Finished`
          (`/Game/Common/SRDisplay/BML_LevelSwitching.SwitchLevel` "kitanaikaku"))))
    (:`B`
      (goto _label :!via `Stop`))))

(event `Reset Animation`
  (goto _label :!via `SetNewTime`))

(fn `UserConstructionScript`)