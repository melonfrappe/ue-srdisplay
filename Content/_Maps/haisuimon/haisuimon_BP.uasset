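; Actor Blueprint for the haisuimon (drainage gate) map that animates a Target actor's yaw and can restore the scene's starting pose.
; DoMove plays a timeline that drives the rotation, then calls SwitchLevel with a None name when finished.
; Stop halts the timeline and Reset sets its time.
; SetDefault restores the Target and ClippingBox transforms cached at BeginPlay; a play/stop FlipFlop is left unwired.
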(event `self.ReceiveBeginPlay`
  (set `self.target_default` (`self.GetTransform` (`self.target`)))
  (set `self.clipping_box_default` (`self.GetTransform` (`self.clipping_box`))))

(event `Do Move`
  (bind (_direction _rotation) (`Timeline|Timeline_0` :!label _label)
    (:`Update`
      (`self.K2_SetActorRotation` (`self.target`) (`KismetMathLibrary.MakeRotator` 0.0 0.0 _rotation) false))
    (:`Finished`
      (`/Game/Common/SRDisplay/BML_LevelSwitching.SwitchLevel` "None"))))

(event `Stop`
  (goto _label :!via `Stop`))

(event `Reset`
  (goto _label :!via `SetNewTime`))

(event `Set Default`
  ;[1 1 1] reset
  (`self.K2_SetActorTransform` (`self.target`) (`self.target_default`) false false)
  (`self.K2_SetActorTransform` (`self.clipping_box`) (`self.clipping_box_default`) false false))

(fn `UserConstructionScript`)