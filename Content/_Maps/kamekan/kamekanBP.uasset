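; Blueprint for the kamekan map that turns a target actor over time, then moves on to the yachiyoza-outside level.
; One second after BeginPlay, a timeline starts driving the target's yaw and switches level when it finishes.
; Separate events stop the timeline, set its time, or restore the transform saved at BeginPlay.
; An unconnected FlipFlop for toggling playback never runs.
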(event `self.ReceiveBeginPlay`
  (set `self.NewVar_0` (`self.GetTransform` (`self.target`)))
  (`KismetSystemLibrary.Delay` 1.0)
  (`self.Do Move`))

(event `Do Move`
  (bind (_direction _rotation) (`Timeline|Timeline_0` :!label _label)
    (:`Update`
      (`self.K2_SetActorRotation` (`self.target`) (`KismetMathLibrary.MakeRotator` 0.0 0.0 _rotation) false))
    (:`Finished`
      (`/Game/Common/SRDisplay/BML_LevelSwitching.SwitchLevel` "yachiyoza-outside"))))

(event `Stop`
  (goto _label :!via `Stop`))

(event `Reset`
  (goto _label :!via `SetNewTime`))

(event `Set Default`
  ;[1 1 1] reset
  (`self.K2_SetActorTransform` (`self.target`) (`self.NewVar_0`) false false))

(fn `UserConstructionScript`)