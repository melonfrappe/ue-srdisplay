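; World-space annotation actor that displays an Annotation through its widget component, using AnnotationWidgetBP, and allows it to be changed via SetAnnotation.
; BeginPlay caches the widget and finds the ControllerBlueprint actor.
; Each Tick it yaws the root toward the controller's SRDisplayManager.
; It also scales itself uniformly by nested square roots of that distance, adjusted by the controller's average NewScale3D, damping size changes.
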(event `self.ReceiveBeginPlay`
  (`|ExecutionSequence`
    (:`then_0`
      (bind _asannotation_widget_bp (cast `/Game/_Maps/plateau/AnnotationWidgetBP` (`WidgetComponent.GetWidget` (`self.Widget`))))
      (bind _output_get (set `self.As Annotation Widget BP` _asannotation_widget_bp))
      (set `/Game/_Maps/plateau/AnnotationWidgetBP.Annotation` (`self.Annotation`) _output_get))
    (:`then_1`
      (bind _returnvalue (`GameplayStatics.GetActorOfClass` "/Game/_Maps/plateau/ControllerBlueprint.ControllerBlueprint_C"))
      (set `self.ControllerBP` _returnvalue))))

(event `Set Annotation`
  (params (Annotation :type Text))
  (set `/Game/_Maps/plateau/AnnotationWidgetBP.Annotation` Annotation (`self.As Annotation Widget BP`)))

(event `self.ReceiveTick`
  (params (DeltaSeconds :type "Float (single-precision)"))
  (bind _defaultsceneroot (`self.DefaultSceneRoot`))
  (bind _returnvalue (`SceneComponent.K2_GetComponentLocation` _defaultsceneroot))
  (bind _ascontroller_blueprint (cast `/Game/_Maps/plateau/ControllerBlueprint` (`self.ControllerBP`)))
  (bind _returnvalue_2 (`self.K2_GetActorLocation` (`/Game/_Maps/plateau/ControllerBlueprint.SRDisplayManager` _ascontroller_blueprint)))
  (bind (_returnvalue_roll _returnvalue_pitch _returnvalue_yaw) (`KismetMathLibrary.BreakRotator` (`KismetMathLibrary.FindLookAtRotation` _returnvalue _returnvalue_2)))
  (`SceneComponent.K2_SetWorldRotation` _defaultsceneroot (`KismetMathLibrary.MakeRotator` 0.0 0.0 _returnvalue_yaw) false false)
  (bind (_new_scale_3d_x _new_scale_3d_y _new_scale_3d_z) (`KismetMathLibrary.BreakVector` (`/Game/_Maps/plateau/ControllerBlueprint.New Scale 3D` _ascontroller_blueprint)))
  (`SceneComponent.SetWorldScale3D` (`self.DefaultSceneRoot`) (`KismetMathLibrary.Conv_DoubleToVector` (`KismetMathLibrary.Sqrt` (`KismetMathLibrary.Sqrt` (/ (`KismetMathLibrary.Vector_Distance` _returnvalue _returnvalue_2) (/ 40.0 (`KismetMathLibrary.Sqrt` (/ (+ _new_scale_3d_x _new_scale_3d_y _new_scale_3d_z) 3.0)))))))))

(fn `UserConstructionScript`)