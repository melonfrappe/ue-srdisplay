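; TargetBP moves a Target along the level's spline path, then hands control back to ControllerBlueprint.
; BeginPlay finds the SplineBP actor, and Move plays a timeline scaled by TimeToComplete to set location and rotation by distance along the spline.
; On finish, it resets the timeline, clears the controller's IsMovingPath flag, increments IndexRotate and calls AutoRotate.
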(event `self.ReceiveBeginPlay`
  (bind _returnvalue (`GameplayStatics.GetActorOfClass` "/Game/_Maps/plateau/SplineBP.SplineBP_C"))
  (set `self.SplineBP` _returnvalue))

(event `Move`
  (bind _spline (`/Game/_Maps/plateau/SplineBP.Spline` (`self.SplineBP`)))
  (`TimelineComponent.SetPlayRate` (`self.Move Object T`) (/ 1.0 (`self.Time To Complete`)))
  (bind (_direction _newtrack_0) (`Timeline|Move Object T` :!label _label)
    (:`Update`
      (bind _returnvalue (`KismetMathLibrary.Lerp` 0.0 (`SplineComponent.GetSplineLength` (`/Game/_Maps/plateau/SplineBP.Spline` (`self.SplineBP`))) _newtrack_0))
      (bind (_returnvalue_roll _returnvalue_pitch _returnvalue_yaw) (`KismetMathLibrary.BreakRotator` (`SplineComponent.GetRotationAtDistanceAlongSpline` _spline _returnvalue "World")))
      (`self.K2_SetActorTransform` (`self.Target`) (`KismetMathLibrary.MakeTransform` (`SplineComponent.GetLocationAtDistanceAlongSpline` _spline _returnvalue "World") (`KismetMathLibrary.MakeRotator` _returnvalue_roll (+ _returnvalue_pitch 0.0) _returnvalue_yaw)) false false))
    (:`Finished`
      (`self.Reset`)
      (bind _returnvalue_2 (`GameplayStatics.GetActorOfClass` "/Game/_Maps/plateau/ControllerBlueprint.ControllerBlueprint_C"))
      (set `/Game/_Maps/plateau/ControllerBlueprint.isMovingPath?` false _returnvalue_2)
      (`/Engine/EditorBlueprintResources/StandardMacros.IncrementInt` (`/Game/_Maps/plateau/ControllerBlueprint.IndexRotate` _returnvalue_2)
        (:`  `
          (`/Game/_Maps/plateau/ControllerBlueprint.Auto-Rotate` _returnvalue_2))))))

(event `Reset`
  (goto _label :!via `SetNewTime`))

(fn `UserConstructionScript`)