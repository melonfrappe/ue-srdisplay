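; Blueprint for the sagara map that plays a scripted movement of a Target actor, then switches to the "plateau" level.
; On BeginPlay it caches the Target's transform and, after a short delay, starts a timeline that drives location, yaw and uniform scale each update.
; Custom events stop or rewind the timeline and restore the cached transform, while some play-toggle logic is left unconnected.
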(event `self.ReceiveBeginPlay`
  (set `self.NewVar_0` (`self.GetTransform` (`self.target`)))
  (`KismetSystemLibrary.Delay` 1.0)
  (`self.Do Move`))

(event `Set Default`
  ;[1 1 1] Comment
  (`self.K2_SetActorTransform` (`self.target`) (`self.NewVar_0`) false false))

(event `Do Move`
  (bind (_direction _rotation _location_x _lcoation_y _location_z _scale) (`Timeline|Timeline_0` :!label _label)
    (:`Update`
      (bind _output_get (set `self.Delta Scale` (`KismetMathLibrary.Conv_DoubleToVector` _scale)))
      (`self.K2_SetActorTransform` (`self.target`) (`KismetMathLibrary.MakeTransform` (`KismetMathLibrary.MakeVector` _location_x _lcoation_y _location_z) (`KismetMathLibrary.MakeRotator` 0.0 0.0 _rotation) _output_get) false false))
    (:`Finished`
      (`/Game/Common/SRDisplay/BML_LevelSwitching.SwitchLevel` "plateau"))))

(event `Stop`
  (goto _label :!via `Stop`))

(event `Reset`
  (goto _label :!via `SetNewTime`))

(fn `UserConstructionScript`)