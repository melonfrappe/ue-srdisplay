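; Yachiyoza interior controller that runs an automated, narrated tour through LiDAR point-cloud floors, then switches to the "plateau" level.
; A timeline, auto-started after a short delay and toggled by DoMove, moves the Target's mesh and reports progress to DynamicContextBP.
; Timeline event tracks trigger indexed 2D sounds, camera-faded floor visibility swaps and SrDisplayManager spatial-clipping toggles.
; Tick keeps the current sound paused whenever the timeline is not playing.
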(event `Set Default`
  ;[1 1 1] reset
  (`self.K2_SetActorTransform` (`self.target`) (`self.defaultTransform`) false false))

(event `self.ReceiveBeginPlay`
  ;[1 1 1] start
  (`|ExecutionSequence`
    (:`then_0`
      (set `self.defaultTransform` (`self.GetTransform` (`self.target`))))
    (:`then_1`
      (bind _returnvalue (`GameplayStatics.GetActorOfClass` "/Game/_Blueprints/DynamicContextBP.DynamicContextBP_C"))
      (set `self.dynamicContext` _returnvalue))
    (:`then_2`
      (`KismetSystemLibrary.Delay` 1.0)
      (`self.Do Move`))))

(event `Play Sound Full`
  (bind _sound (`self.sound`))
  ;[1 1 1] play pause
  (`/Engine/EditorBlueprintResources/StandardMacros.IsValid` (`self.sound`)
    (:`Is Valid`
      (`/Engine/EditorBlueprintResources/StandardMacros.FlipFlop`
        (:`A`
          (`AudioComponent.SetPaused` _sound true))
        (:`B`
          (`AudioComponent.SetPaused` _sound false))))
    (:`Is Not Valid`
      (bind _returnvalue (`GameplayStatics.SpawnSound2D` (`self.audio_full`) 1.0 1.0 0.0 null))
      (set `self.sound` _returnvalue))))

(event `Play Sound Index`
  (params (Index :type Integer))
  ;[1 1 1] play index
  (bind _returnvalue (`GameplayStatics.SpawnSound2D` (`|GetArrayItem` (`self.audios`) Index) 1.0 1.0 0.0 null))
  (set `self.sound` _returnvalue))

(event `Do Move`
  (bind _timeline_0 (`self.Timeline_0`))
  ;[1 1 1] Comment
  (if (`self.isFinished?`)
    (`self.Reset Move`))
  (if (`self.isMove?`)
    (set `self.isMove?` false :!label _label)
    (bind (_direction _location _rotation _scale) (`Timeline|Timeline_0` :!via `Stop` :!label _label_2)
      (:`Update`
        (`SceneComponent.K2_SetWorldTransform` (`StaticMeshActor.StaticMeshComponent` (`self.target`)) (`KismetMathLibrary.MakeTransform` _location (`KismetMathLibrary.MakeRotator` (.x _rotation) (.y _rotation) (.z _rotation)) (`KismetMathLibrary.Conv_DoubleToVector` _scale)) false false)
        (`/Game/_Blueprints/DynamicContextBP.Set Progress` (`self.dynamicContext`) (/ (`TimelineComponent.GetPlaybackPosition` _timeline_0) (`TimelineComponent.GetTimelineLength` _timeline_0))))
      (:`Finished`
        (set `self.isFinished?` true)
        (set `self.isMove?` false)
        (`/Game/Common/SRDisplay/BML_LevelSwitching.SwitchLevel` "plateau"))
      (:`to 2F`
        (`self.Toggle Floor` 1))
      (:`to 3F`
        (`self.Toggle Floor` 2))
      (:`toggle clipping`
        (`self.Toggle Clipping`))
      (:`play sound 0`
        (`self.Play Sound Index` 0))
      (:`play sound 1`
        (`self.Play Sound Index` 1))
      (:`play sound 2`
        (`self.Play Sound Index` 2))
      (:`play sound 3`
        (`self.Play Sound Index` 3))
      (:`play sound 4`
        (`self.Play Sound Index` 4))
      (:`play sound 5`
        (`self.Play Sound Index` 5))
      (:`play sound 6`
        (`self.Play Sound Index` 6))
      (:`play sound 7`
        (`self.Play Sound Index` 7))
      (:`play sound 8`
        (`self.Play Sound Index` 8))
      (:`play sound 9`
        (`self.Play Sound Index` 9))
      (:`play sound 10`
        (`self.Play Sound Index` 10)))
    (else
      (set `self.isMove?` true)
      (goto _label_2))))

(event `Stop Move`
  ;[1 1 1] Comment
  (goto _label))

(event `Reset Move`
  ;[1 1 1] Comment
  (set `self.isFinished?` false)
  (`self.Toggle Floor` 0)
  (goto _label_2 :!via `SetNewTime`))

(event `Stop Sound`
  (bind _sound (`self.sound`))
  ;[1 1 1] stop sound
  (`/Engine/EditorBlueprintResources/StandardMacros.IsValid` _sound
    (:`Is Valid`
      (`AudioComponent.Stop` _sound))))

(event `Toggle Floor`
  (params (Index :type Integer))
  (bind _lidaractor (`self.lidarActor`))
  ;[1 1 1] toggle floor
  (`PlayerCameraManager.StartCameraFade` :`self` (`GameplayStatics.GetPlayerCameraManager` 0) :`ToAlpha` 1.0 :`Duration` 0.5 :`bHoldWhenFinished` true)
  (`KismetSystemLibrary.Delay` 0.5)
  (`SceneComponent.SetVisibility` (`LidarPointCloudActor.PointCloudComponent` (`|GetArrayItem` _lidaractor Index)) true false)
  (for (_array_element _array_index) _lidaractor
    (`SceneComponent.SetVisibility` (`LidarPointCloudActor.PointCloudComponent` _array_element) (== _array_index Index) true)
    (`PlayerCameraManager.StartCameraFade` :`self` (`GameplayStatics.GetPlayerCameraManager` 0) :`FromAlpha` 1.0 :`Duration` 0.5)))

(event `Toggle Clipping`
  (bind _srdisplaymanager (`self.srDisplayManager`))
  ;[1 1 1] set clipping
  (set `SRDisplayManager.SpatialClipping` (not (`SRDisplayManager.SpatialClipping` _srdisplaymanager)) _srdisplaymanager))

(event `self.ReceiveTick`
  (params (DeltaSeconds :type "Float (single-precision)"))
  (bind _sound (`self.sound`))
  (`/Engine/EditorBlueprintResources/StandardMacros.IsValid` _sound
    (:`Is Valid`
      (`AudioComponent.SetPaused` _sound (not (`TimelineComponent.IsPlaying` (`self.Timeline_0`)))))))

(fn `UserConstructionScript`)