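; Outside-scene controller for the Yachiyoza map that plays a timed transform animation on a target actor, then switches to the yachiyoza-inside level.
; DoMove starts automatically one second after BeginPlay and toggles play/stop, resetting the timeline if finished.
; Timeline_1 drives location, rotation and scale, reports progress to DynamicContextBP, and fires events for 2D audio and SR display spatial-clipping toggles.
; Tick pauses the audio whenever the timeline is not playing.
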(event `self.ReceiveBeginPlay`
  ;[1 1 1] start
  (`|ExecutionSequence`
    (:`then_0`
      (set `self.defaultTransform` (`self.GetTransform` (`self.target`))))
    (:`then_1`
      (bind _returnvalue (`GameplayStatics.GetActorOfClass` "/Game/_Blueprints/DynamicContextBP.DynamicContextBP_C"))
      (set `self.dynamicContext` _returnvalue))
    (:`then_2`
      (`KismetSystemLibrary.Delay` 1.0)
      (`self.Do Move`))))

(event `Set Default`
  ;[1 1 1] reset
  (`self.K2_SetActorTransform` (`self.target`) (`self.defaultTransform`) false false))

(event `Do Move`
  (bind _timeline_1 (`self.Timeline_1`))
  ;[1 1 1] move
  (if (`self.isFinished?`)
    (set `self.isFinished?` false)
    (`self.Reset Move`))
  (if (`self.isMove?`)
    (set `self.isMove?` false :!label _label)
    (bind (_direction _location _rotation _scale) (`Timeline|Timeline_1` :!via `Stop` :!label _label_2)
      (:`Update`
        (`self.K2_SetActorTransform` (`self.target`) (`KismetMathLibrary.MakeTransform` _location (`KismetMathLibrary.MakeRotator` (.x _rotation) (.y _rotation) (.z _rotation)) (`KismetMathLibrary.Conv_DoubleToVector` _scale)) false false)
        (`/Game/_Blueprints/DynamicContextBP.Set Progress` (`self.dynamicContext`) (/ (`TimelineComponent.GetPlaybackPosition` _timeline_1) (`TimelineComponent.GetTimelineLength` _timeline_1))))
      (:`Finished`
        (set `self.isMove?` false)
        (set `self.isFinished?` true)
        (`/Game/Common/SRDisplay/BML_LevelSwitching.SwitchLevel` "yachiyoza-inside"))
      (:`play sound`
        (`self.Play Sound All`))
      (:`toggle clippling`
        (`self.Toggle Clipping`)))
    (else
      (set `self.isMove?` true)
      (goto _label_2))))

(event `Stop Move`
  ;[1 1 1] move
  (goto _label))

(event `Reset Move`
  ;[1 1 1] move
  (goto _label_2 :!via `SetNewTime`))

(event `Play Sound All`
  ;[1 1 1] play
  (bind _returnvalue (`GameplayStatics.SpawnSound2D` (`self.audio_full`) 1.0 1.0 0.0 null))
  (set `self.sound` _returnvalue))

(event `Stop Sound`
  (bind _sound (`self.sound`))
  ;[1 1 1] stop sound
  (`/Engine/EditorBlueprintResources/StandardMacros.IsValid` _sound
    (:`Is Valid`
      (`AudioComponent.Stop` _sound))))

(event `self.ReceiveTick`
  (params (DeltaSeconds :type "Float (single-precision)"))
  (bind _sound (`self.sound`))
  (`/Engine/EditorBlueprintResources/StandardMacros.IsValid` _sound
    (:`Is Valid`
      (`AudioComponent.SetPaused` _sound (not (`TimelineComponent.IsPlaying` (`self.Timeline_1`)))))))

(event `Toggle Clipping`
  (bind _srdisplaymanager (`self.srDisplayManager`))
  ;[1 1 1] set clipping
  (set `SRDisplayManager.SpatialClipping` (not (`SRDisplayManager.SpatialClipping` _srdisplaymanager)) _srdisplaymanager))

(fn `UserConstructionScript`)